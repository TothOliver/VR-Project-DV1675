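; BP_KassaPoint is a checkout (kassa) spot that a customer can claim, holding a single Occupied flag.
; On BeginPlay it registers itself in the game instance's KassaARRAY at its KassaPointID index.
; TryOccupy refuses if taken; otherwise it occupies itself, frees the point at the requesting customer's CurrentSpot index with debug prints, and returns true.
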(event EventBeginPlay
  (bind _asbp_game_instance (Utilities|Casting|CastToBP_GameInstance (Game|GetGameInstance)))
  (Utilities|Array|SetArrayElem (Variables|/Game/Blueprints/BP_GameInstance.BP_GameInstance_C|GetKassaARRAY _asbp_game_instance) (Variables|Default|GetKassaPoint_ID) self true))

(event Collision|EventActorBeginOverlap
  (params (OtherActor :type Actor%20Object%20Reference)))

(event EventTick
  (params (DeltaSeconds :type Float%20%28single-precision%29)))

(fn ConstructionScript)

(fn TryOccupy
  (params (RequestingCustomer :type BP%20Customer%20Object%20Reference))
  (if (Variables|Default|GetOccupied)
    (return false)
    (else
      (Variables|Default|SetOccupied true)
      (bind _asbp_game_instance (Utilities|Casting|CastToBP_GameInstance (Game|GetGameInstance)))
      (bind (_array_element _array_index) (Utilities|Array|ForEachLoopwithBreak (Variables|/Game/Blueprints/BP_GameInstance.BP_GameInstance_C|GetKassaARRAY _asbp_game_instance) :!label _label)
        (:LoopBody
          (if (== _array_index (Variables|/Game/Blueprints/Customer/BP_Customer.BP_Customer_C|GetCurrentSpot RequestingCustomer))
            (Variables|BP_KassaPoint_C|SetOccupied _array_element false)
            (Development|PrintString (Utilities|GetDisplayName _array_element))
            (Development|PrintString "No longer occupied")
            (goto _label Break)))
        (:Completed
          (return true))))))