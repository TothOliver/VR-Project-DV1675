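; BP_Customer is an AI customer character that orders at a register and leaves for an end point.
; Interacting while CurrentSpot is 0 sets the IsMakingOrder blackboard key and frees the first KassaARRAY spot in BP_GameInstance.
; ReturnToCar uses AIMoveTo toward BP_EndPoint actors, then rotates the capsule on arrival.
; Unconnected leftover logic covers walking to BP_KassaPoint, posting WB_Orders orders and approaching the player.
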(event OnSeePawn(PawnSensing)
  (params (Pawn :type Pawn%20Object%20Reference)))

(event Custom|ReturnToCar
  (bind _outactors (Actor|GetAllActorsOfClass "/Game/Blueprints/Customer/BP_EndPoint.BP_EndPoint_C"))
  (for _array_element _outactors
    (AI|AIMoveTo self (Transformation|GetActorLocation _array_element) 0 5.0 false
      (:OnSuccess
        (Transformation|SetWorldRotation (Variables|Collision|GetCapsuleComponent) "0.000000,-90.000000,0.000000" false false)))))

(event EventBeginPlay)

(event Collision|EventActorBeginOverlap
  (params (OtherActor :type Actor%20Object%20Reference)))

(event EventTick
  (params (DeltaSeconds :type Float%20%28single-precision%29)))

(event EventOnCustomerInteracted
  (if (== (Variables|Default|GetCurrentSpot) 0)
    (AI|Components|Blackboard|SetValueasBool (AI|GetBlackboard 0) (Utilities|Name|MakeLiteralName "IsMakingOrder") true)
    (bind _asbp_game_instance (Utilities|Casting|CastToBP_GameInstance (Game|GetGameInstance)))
    (bind (_array_element _array_index) (Utilities|Array|ForEachLoopwithBreak (Variables|/Game/Blueprints/BP_GameInstance.BP_GameInstance_C|GetKassaARRAY _asbp_game_instance))
      (:LoopBody
        (if (== _array_index 0)
          (Variables|/Game/Blueprints/Customer/BP_KassaPoint.BP_KassaPoint_C|SetOccupied _array_element false))))
    (else
      (Development|PrintString "Failed here?"))))

(fn ConstructionScript)