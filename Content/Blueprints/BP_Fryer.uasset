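; BP_Fryer is a fryer actor that detects fryer baskets and snaps them into set positions.
; Four overlap volumes, left and right both in oil and above, pass their target point to SnapPosition.
; If the basket is not held when the overlap begins, SnapPosition disables its mesh physics and teleports the overlapping component to that point with zeroed rotation.
; A separate SnapZone overlap sets and clears CurrentBasket.
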(event OnComponentBeginOverlap(SnapZone)
  (params (OverlappedComponent :type Primitive%20Component%20Object%20Reference) (OtherActor :type Actor%20Object%20Reference) (OtherComp :type Primitive%20Component%20Object%20Reference) (OtherBodyIndex :type Integer) (bFromSweep :type Boolean) (SweepResult :type Hit%20Result%20Structure%20%28by%20ref%29))
  (bind _asbp_fryer_basket (Utilities|Casting|CastToBP_FryerBasket OtherActor))
  (Variables|Default|SetCurrentBasket _asbp_fryer_basket)
  (Development|PrintString "Basket Detected"))

(event OnComponentEndOverlap(SnapZone)
  (params (OverlappedComponent :type Primitive%20Component%20Object%20Reference) (OtherActor :type Actor%20Object%20Reference) (OtherComp :type Primitive%20Component%20Object%20Reference) (OtherBodyIndex :type Integer))
  (Utilities|Casting|CastToBP_FryerBasket OtherActor)
  (Variables|Default|SetCurrentBasket 0))

(event OnComponentBeginOverlap(Snap_Left_InOil)
  (params (OverlappedComponent :type Primitive%20Component%20Object%20Reference) (OtherActor :type Actor%20Object%20Reference) (OtherComp :type Primitive%20Component%20Object%20Reference) (OtherBodyIndex :type Integer) (bFromSweep :type Boolean) (SweepResult :type Hit%20Result%20Structure%20%28by%20ref%29))
  (CallFunction|SnapPosition OtherActor OtherComp (Variables|Default|GetSP_Left_InOil)))

(event OnComponentBeginOverlap(Snap_Right_InOil)
  (params (OverlappedComponent :type Primitive%20Component%20Object%20Reference) (OtherActor :type Actor%20Object%20Reference) (OtherComp :type Primitive%20Component%20Object%20Reference) (OtherBodyIndex :type Integer) (bFromSweep :type Boolean) (SweepResult :type Hit%20Result%20Structure%20%28by%20ref%29))
  (CallFunction|SnapPosition OtherActor OtherComp (Variables|Default|GetSP_Right_InOil)))

(event OnComponentBeginOverlap(Snap_Left_Above)
  (params (OverlappedComponent :type Primitive%20Component%20Object%20Reference) (OtherActor :type Actor%20Object%20Reference) (OtherComp :type Primitive%20Component%20Object%20Reference) (OtherBodyIndex :type Integer) (bFromSweep :type Boolean) (SweepResult :type Hit%20Result%20Structure%20%28by%20ref%29))
  (CallFunction|SnapPosition OtherActor OtherComp (Variables|Default|GetSP_Left_Above)))

(event OnComponentBeginOverlap(Snap_Right_Above)
  (params (OverlappedComponent :type Primitive%20Component%20Object%20Reference) (OtherActor :type Actor%20Object%20Reference) (OtherComp :type Primitive%20Component%20Object%20Reference) (OtherBodyIndex :type Integer) (bFromSweep :type Boolean) (SweepResult :type Hit%20Result%20Structure%20%28by%20ref%29))
  (CallFunction|SnapPosition OtherActor OtherComp (Variables|Default|GetSP_Right_Above)))

(event EventBeginPlay)

(event Collision|EventActorBeginOverlap
  (params (OtherActor :type Actor%20Object%20Reference)))

(event EventTick
  (params (DeltaSeconds :type Float%20%28single-precision%29)))

(fn ConstructionScript)

(fn SnapPosition
  (params (Other%20Actor :type Actor%20Object%20Reference) (Other%20Comp :type Primitive%20Component%20Object%20Reference) (SP_Position :type Arrow%20Component%20Object%20Reference))
  (bind _asbp_fryer_basket (Utilities|Casting|CastToBP_FryerBasket Other%20Actor))
  (if (not (Variables|/Game/XRFramework/Blueprints/BP_GrabComponent.BP_GrabComponent_C|GetbIsHeld (Actor|GetComponentbyClass _asbp_fryer_basket "/Game/XRFramework/Blueprints/BP_GrabComponent.BP_GrabComponent_C")))
    (Physics|SetSimulatePhysics (Variables|/Game/Blueprints/BP_FryerBasket.BP_FryerBasket_C|GetRaw_meat_Foods_07_0 _asbp_fryer_basket) false)
    (Transformation|SetWorldRotation Other%20Comp "0, 0, 0" false true)
    (Transformation|SetWorldLocation Other%20Comp (Transformation|GetWorldLocation SP_Position) false true)))