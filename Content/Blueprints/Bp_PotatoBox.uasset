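; BP_PotatoBox is a VR potato dispenser that spawns a new potato when its grab handle is grabbed.
; BeginPlay caches the player's BP_XRPawn.
; On grab, it spawns a BP_GrabPotato at the GrabMeshHandle transform, even if colliding.
; It then checks which hand holds the handle and attaches the potato to the pawn's matching left or right held component, keeping relative transforms.
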(event OnGrabbed(GrabHandle)
  (Utilities|IsValid (Variables|Default|GetXRPawnref)
    (:Is%20Valid
      (bind _returnvalue (Game|SpawnActorfromClass "/Game/Blueprints/BP_GrabPotato.BP_GrabPotato_C" (Transformation|GetWorldTransform (Variables|Default|GetGrabMeshHandle)) "AlwaysSpawn" "MultiplyWithRoot" 0 0))
      (switch Utilities|FlowControl|Switch|SwitchonEControllerHand (Default|GetHeldbyHand (Variables|Default|GetGrabHandle))
        (:Left
          (Transformation|AttachComponentToComponent _returnvalue (Variables|/Game/XRFramework/Blueprints/BP_XRPawn.BP_XRPawn_C|GetHeldComponentLeft (Variables|Default|GetXRPawnref)) "None" "KeepRelative" "KeepRelative" "KeepRelative" true))
        (:Right
          (Transformation|AttachComponentToComponent _returnvalue (Variables|/Game/XRFramework/Blueprints/BP_XRPawn.BP_XRPawn_C|GetHeldComponentRight (Variables|Default|GetXRPawnref)) "None" "KeepRelative" "KeepRelative" "KeepRelative" true))))))

(event EventBeginPlay
  (bind _asbp_xrpawn (Utilities|Casting|CastToBP_XRPawn (Pawn|GetControlledPawn (Game|GetPlayerController 0))))
  (Variables|Default|SetXRPawnref _asbp_xrpawn))

(event Collision|EventActorBeginOverlap
  (params (OtherActor :type Actor%20Object%20Reference)))

(event EventTick
  (params (DeltaSeconds :type Float%20%28single-precision%29)))

(fn ConstructionScript)