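; BP_CashRegister is a cash register actor that relays an interaction to customers standing at register spots.
; On OnCustomerInteracted, it loops over the game instance's KassaARRAY and searches all BP_Customer actors for each entry.
; Every customer whose CurrentSpot matches an entry's KassaPointID receives OnCustomerInteracted, with a 2D cashier beep per match.
; The match covers all register points, not just this register's own.
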(event EventBeginPlay)

(event Collision|EventActorBeginOverlap
  (params (OtherActor :type Actor%20Object%20Reference)))

(event EventTick
  (params (DeltaSeconds :type Float%20%28single-precision%29)))

(event EventOnCustomerInteracted
  (bind _asbp_game_instance (Utilities|Casting|CastToBP_GameInstance (Game|GetGameInstance)))
  (bind _array_element (Utilities|Array|ForEachLoopwithBreak (Variables|/Game/Blueprints/BP_GameInstance.BP_GameInstance_C|GetKassaARRAY _asbp_game_instance))
    (:LoopBody
      (bind _outactors (Actor|GetAllActorsOfClass "/Game/Blueprints/Customer/BP_Customer.BP_Customer_C"))
      (for _array_element_2 _outactors
        (if (== (Variables|/Game/Blueprints/Customer/BP_KassaPoint.BP_KassaPoint_C|GetKassaPoint_ID _array_element) (Variables|/Game/Blueprints/Customer/BP_Customer.BP_Customer_C|GetCurrentSpot _array_element_2))
          (Default|OnCustomerInteracted _array_element_2)
          (Audio|PlaySound2D "/Game/Blueprints/Sounds/CasheirBeep_Cue.CasheirBeep_Cue" 1.0 1.0 0.0 0 0))))))

(fn ConstructionScript)