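; BP_DoubleDoor is a double door that opens automatically for BP_Customer actors.
; The CollisionCheck overlap events call DoorMagic, guarded by an Open flag, with a short delay before closing.
; DoorMagic uses a FlipFlop to alternate between opening and closing, toggling door mesh collision.
; A timeline lerps two arrow components' yaw in opposite directions, playing forward to open and reversing from the end to close.
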(event OnComponentBeginOverlap(CollisionCheck)
  (params (OverlappedComponent :type Primitive%20Component%20Object%20Reference) (OtherActor :type Actor%20Object%20Reference) (OtherComp :type Primitive%20Component%20Object%20Reference) (OtherBodyIndex :type Integer) (bFromSweep :type Boolean) (SweepResult :type Hit%20Result%20Structure%20%28by%20ref%29))
  (Utilities|Casting|CastToBP_Customer OtherActor)
  (if (not (Variables|Default|GetOpen))
    (CallFunction|DoorMagic)
    (Variables|Default|SetOpen true)))

(event OnComponentEndOverlap(CollisionCheck)
  (params (OverlappedComponent :type Primitive%20Component%20Object%20Reference) (OtherActor :type Actor%20Object%20Reference) (OtherComp :type Primitive%20Component%20Object%20Reference) (OtherBodyIndex :type Integer))
  (Utilities|Casting|CastToBP_Customer OtherActor)
  (if (Variables|Default|GetOpen)
    (Utilities|FlowControl|Delay 0.2)
    (CallFunction|DoorMagic)
    (Variables|Default|SetOpen false)))

(event Custom|DoorMagic
  (bind _door_f_001 (Variables|Default|GetDoor_F_001))
  (Utilities|FlowControl|FlipFlop
    (:A
      (Collision|SetCollisionEnabled _door_f_001 "NoCollision")
      (bind _newtrack_0 (Timeline|Timeline Play)
        (:Update
          (Transformation|SetRelativeRotation (Variables|Default|GetArrow) (Math|Rotator|Lerp(Rotator) "0, 0, 0" "0.000000,-90.000000,0.000000" _newtrack_0) false false)
          (Transformation|SetRelativeRotation (Variables|Default|GetArrow1) (Math|Rotator|Lerp(Rotator) "0, 0, 0" "0.000000,90.000000,0.000000" _newtrack_0) false false))))
    (:B
      (Collision|SetCollisionEnabled _door_f_001 "QueryAndPhysics")
      (Timeline|Timeline ReverseFromEnd))))

(event EventBeginPlay)

(event Collision|EventActorBeginOverlap
  (params (OtherActor :type Actor%20Object%20Reference)))

(event EventTick
  (params (DeltaSeconds :type Float%20%28single-precision%29)))

(fn ConstructionScript)