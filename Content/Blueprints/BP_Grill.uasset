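; BP_Grill is a grill actor that cooks burgers placed on it and plays a sizzling sound.
; Box overlap events cast the other actor to BP_CookedBurger and start or stop cooking on its Burger component.
; A BurgersOnGrill counter plays the sizzle cue when the first burger arrives and fades it out when the last one leaves.
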(event OnComponentEndOverlap(Box)
  (params (OverlappedComponent :type Primitive%20Component%20Object%20Reference) (OtherActor :type Actor%20Object%20Reference) (OtherComp :type Primitive%20Component%20Object%20Reference) (OtherBodyIndex :type Integer))
  (bind _asbp_cooked_burger (Utilities|Casting|CastToBP_CookedBurger OtherActor))
  (Class|BurgerComponent|StopCooking (Variables|/Game/Blueprints/BP_CookedBurger.BP_CookedBurger_C|GetBurger _asbp_cooked_burger))
  ;[0.15 0.15 0.15 0.5] Handles the Sizzling sound on the Grill
  (Variables|Default|SetBurgersOnGrill (- (Variables|Default|GetBurgersOnGrill) 1))
  (if (== (Variables|Default|GetBurgersOnGrill) 0)
    (Audio|Components|Audio|FadeOut (Variables|Default|GetSizzlingSound_Cue) 0.5 0.0 "Linear" :!class /Script/Engine.AudioComponent)))

(event OnComponentBeginOverlap(Box)
  (params (OverlappedComponent :type Primitive%20Component%20Object%20Reference) (OtherActor :type Actor%20Object%20Reference) (OtherComp :type Primitive%20Component%20Object%20Reference) (OtherBodyIndex :type Integer) (bFromSweep :type Boolean) (SweepResult :type Hit%20Result%20Structure%20%28by%20ref%29))
  (bind _asbp_cooked_burger (Utilities|Casting|CastToBP_CookedBurger OtherActor))
  (Class|BurgerComponent|StartCooking (Variables|/Game/Blueprints/BP_CookedBurger.BP_CookedBurger_C|GetBurger _asbp_cooked_burger))
  ;[0.15 0.15 0.15 0.5] Handles the Sizzling sound on the Grill
  (Variables|Default|SetBurgersOnGrill (+ (Variables|Default|GetBurgersOnGrill) 1))
  (if (== (Variables|Default|GetBurgersOnGrill) 1)
    (Audio|Components|Audio|Play (Variables|Default|GetSizzlingSound_Cue) 0.0)))

(event EventBeginPlay)

(event Collision|EventActorBeginOverlap
  (params (OtherActor :type Actor%20Object%20Reference)))

(event EventTick
  (params (DeltaSeconds :type Float%20%28single-precision%29)))

(fn ConstructionScript)

(fn NewFunction)