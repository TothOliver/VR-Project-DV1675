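; BP_Car01 is an AI-moved car pawn that drives to an end point and drops off a customer.
; On BeginPlay it loops over all BP_EndPoint actors, issuing an AIMoveTo toward each location without waiting between iterations.
; On a successful move, it snaps its capsule to a fixed rotation and spawns a BP_Customer at a fixed world-space offset beside it.
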(event EventBeginPlay
  (bind _capsulecomponent (Variables|Collision|GetCapsuleComponent))
  (bind _outactors (Actor|GetAllActorsOfClass "/Game/Blueprints/Customer/BP_EndPoint.BP_EndPoint_C"))
  (for _array_element _outactors
    (AI|AIMoveTo self (Transformation|GetActorLocation _array_element) 0 5.0 false
      (:OnSuccess
        (Transformation|SetWorldRotation _capsulecomponent "0.000000,-90.000000,0.000000" false false)
        (Game|SpawnActorfromClass "/Game/Blueprints/Customer/BP_Customer.BP_Customer_C" (Math|Conversions|ToTransform(Vector) (- (Transformation|GetWorldLocation _capsulecomponent) "0.000000,400.000000,0.000000")) "AdjustIfPossibleButAlwaysSpawn" "MultiplyWithRoot" 0 0)))))

(event Collision|EventActorBeginOverlap
  (params (OtherActor :type Actor%20Object%20Reference)))

(event EventTick
  (params (DeltaSeconds :type Float%20%28single-precision%29)))

(fn ConstructionScript)