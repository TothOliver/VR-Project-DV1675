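; BP_FryerBasket is a grabbable fryer basket that holds and cooks potatoes.
; Uncooked BP_GrabPotato actors entering PotatoZone stop simulating physics, attach to it and join PotatoesInBasket.
; StartCookingPotato, while IsInOil is set, adds cook time to each potato on a self-set looping timer; StopCookingPotato releases cooked ones with physics restored.
; Grabbing clears IsInOil and disables collision until dropped; nothing here sets IsInOil true.
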(event OnDropped(BP_GrabComponent)
  (Collision|SetActorEnableCollision true))

(event OnGrabbed(BP_GrabComponent)
  (Variables|Default|SetIsInOil false)
  (Collision|SetActorEnableCollision false))

(event OnComponentBeginOverlap(PotatoZone)
  (params (OverlappedComponent :type Primitive%20Component%20Object%20Reference) (OtherActor :type Actor%20Object%20Reference) (OtherComp :type Primitive%20Component%20Object%20Reference) (OtherBodyIndex :type Integer) (bFromSweep :type Boolean) (SweepResult :type Hit%20Result%20Structure%20%28by%20ref%29))
  (bind _asbp_grab_potato (Utilities|Casting|CastToBP_GrabPotato OtherActor))
  (if (not (Variables|/Game/Blueprints/BP_GrabPotato.BP_GrabPotato_C|GetIsCooked _asbp_grab_potato))
    (Physics|SetSimulatePhysics (Variables|/Game/Blueprints/BP_GrabPotato.BP_GrabPotato_C|GetPotato _asbp_grab_potato) false)
    (Transformation|AttachComponentToComponent _asbp_grab_potato (Variables|Default|GetPotatoZone) "None" "SnapToTarget" "KeepWorld" "KeepWorld" false)
    (Utilities|Array|Add (Variables|Default|GetPotatoesInBasket) _asbp_grab_potato)))

(event Custom|StopCookingPotato
  (CallFunction|StopCooking))

(event Custom|StartCookingPotato
  (if (Variables|Default|GetIsInOil)
    (CallFunction|CookPotato)
    (Utilities|Time|SetTimerbyEvent (delegate Custom|StartCookingPotato) 0.2 true true)))

(event EventBeginPlay)

(event Collision|EventActorBeginOverlap
  (params (OtherActor :type Actor%20Object%20Reference)))

(event EventTick
  (params (DeltaSeconds :type Float%20%28single-precision%29)))

(fn ConstructionScript)

(fn CookPotato
  (for _array_element (Variables|Default|GetPotatoesInBasket)
    (Default|AddCookTime _array_element)))

(fn StopCooking
  (for _array_element (Variables|Default|GetPotatoesInBasket)
    (if (Variables|/Game/Blueprints/BP_GrabPotato.BP_GrabPotato_C|GetIsCooked _array_element)
      (Transformation|DetachFromActor _array_element "KeepWorld" "KeepWorld" "KeepWorld")
      (Physics|SetSimulatePhysics (Variables|/Game/Blueprints/BP_GrabPotato.BP_GrabPotato_C|GetPotato _array_element) true)
      (Utilities|Array|RemoveItem (Variables|Default|GetPotatoesInBasket) _array_element))))