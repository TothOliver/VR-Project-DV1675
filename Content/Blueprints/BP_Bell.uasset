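; BP_Bell is a service bell that hands in food orders when its OnCustomerInteracted event fires.
; It compares each BP_Tray's hamburger, fries and potato contents with the pending orders in WB_Orders widgets.
; On a match, it finds the BP_Customer by order ID, sets its OrderComplete blackboard key, removes the order and resets the tray.
; All lookups use world-wide actor and widget searches, with debug prints left in.
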(event OnGrabbed(BP_GrabComponent))

(event EventBeginPlay)

(event Collision|EventActorBeginOverlap
  (params (OtherActor :type Actor%20Object%20Reference)))

(event EventTick
  (params (DeltaSeconds :type Float%20%28single-precision%29)))

(event EventOnCustomerInteracted
  (bind _outactors (Actor|GetAllActorsOfClass "/Game/Blueprints/BP_Tray.BP_Tray_C"))
  (for _array_element _outactors
    (Development|PrintString (Utilities|String|Append (Utilities|String|ToString(Boolean) (.hamburger (Variables|/Game/Blueprints/BP_Tray.BP_Tray_C|GetCurrentOrderOnTray _array_element))) (Utilities|String|ToString(Boolean) (.fries (Variables|/Game/Blueprints/BP_Tray.BP_Tray_C|GetCurrentOrderOnTray _array_element))) (Utilities|String|ToString(Boolean) (.potato (Variables|/Game/Blueprints/BP_Tray.BP_Tray_C|GetCurrentOrderOnTray _array_element)))))
    (bind _foundwidgets (Widget|GetAllWidgetsOfClass "/Game/Widgets/WB_Orders.WB_Orders_C" false))
    (for _array_element_2 _foundwidgets
      (for (_array_element_3 _array_index) (Variables|/Game/Widgets/WB_Orders.WB_Orders_C|GetNewOrders _array_element_2)
        (if (== (.Hamburger (Utilities|Struct|BreakS_FoodOrder _array_element_3)) (.hamburger (Variables|/Game/Blueprints/BP_Tray.BP_Tray_C|GetCurrentOrderOnTray _array_element)))
          (if (== (.Fries (Utilities|Struct|BreakS_FoodOrder _array_element_3)) (.fries (Variables|/Game/Blueprints/BP_Tray.BP_Tray_C|GetCurrentOrderOnTray _array_element)))
            (if (== (.Potato (Utilities|Struct|BreakS_FoodOrder _array_element_3)) (.potato (Variables|/Game/Blueprints/BP_Tray.BP_Tray_C|GetCurrentOrderOnTray _array_element)))
              (bind _outactors_2 (Actor|GetAllActorsOfClass "/Game/Blueprints/Customer/BP_Customer.BP_Customer_C"))
              (bind _array_element_4 (Utilities|Array|ForEachLoopwithBreak _outactors_2 :!label _label)
                (:LoopBody
                  (if (== (Variables|/Game/Blueprints/Customer/BP_Customer.BP_Customer_C|GetCustomerID _array_element_4) (.OrderID (Utilities|Struct|BreakS_FoodOrder _array_element_3)))
                    (goto _label Break)))
                (:Completed
                  (Development|PrintString "Hello")
                  (AI|Components|Blackboard|SetValueasBool (AI|GetBlackboard _array_element_4) (Utilities|Name|MakeLiteralName "OrderComplete") true)
                  (Utilities|Array|RemoveIndex (Variables|/Game/Widgets/WB_Orders.WB_Orders_C|GetNewOrders _array_element_2) _array_index)
                  (Variables|/Game/Blueprints/BP_Tray.BP_Tray_C|SetCurrentOrderOnTray _array_element (Utilities|Struct|MakeS_FoodOrder false false false 1000)))))))))))

(fn ConstructionScript)