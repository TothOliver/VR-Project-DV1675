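; TestActor01 is a test snap-point actor that catches an overlapping TestActor02 and attaches it to SnapPointTop.
; Box and Cube overlaps run the snap when neither actor is grabbed, disabling the sphere's physics and collision and changing its grab type.
; Setting CollisionEnabled triggers an OnRep that reapplies the physics and collision shutdown to the stored sphere reference.
; Customer interaction toggles this actor's IsGrabbed flag, while player-detach logic sits unconnected.
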(event OnComponentBeginOverlap(Cube)
  (params (OverlappedComponent :type Primitive%20Component%20Object%20Reference) (OtherActor :type Actor%20Object%20Reference) (OtherComp :type Primitive%20Component%20Object%20Reference) (OtherBodyIndex :type Integer) (bFromSweep :type Boolean) (SweepResult :type Hit%20Result%20Structure%20%28by%20ref%29))
  (bind _astest_actor_02 (Utilities|Casting|CastToTestActor02 (stale Custom|TEstOverlap OverlappedActor)))
  (Variables|Default|SetSphereREF _astest_actor_02)
  (bind _asbp_first_person_character (Utilities|Casting|CastToBP_FirstPersonCharacter (Game|GetPlayerCharacter 0)))
  (if (not (Variables|Default|GetIsGrabbed))
    (if (not (Variables|/Game/Blueprints/TestActor02.TestActor02_C|GetIsGrabbed _astest_actor_02))
      (Physics|SetSimulatePhysics (Variables|/Game/Blueprints/TestActor02.TestActor02_C|GetSPhere _astest_actor_02) false)
      (Variables|/Game/XRFramework/Blueprints/BP_GrabComponent.BP_GrabComponent_C|SetGrabType (Variables|/Game/Blueprints/TestActor02.TestActor02_C|GetBP_GrabComponent _astest_actor_02) "NewEnumerator0")
      (Collision|SetCollisionEnabled (Variables|/Game/Blueprints/TestActor02.TestActor02_C|GetSPhere _astest_actor_02) "NoCollision")
      (Variables|Default|SetCollisionEnabled true)
      (Transformation|AttachComponentToComponent _astest_actor_02 (Variables|Default|GetSnapPoint_Top) "None" "SnapToTarget" "SnapToTarget" "KeepWorld" true))))

(event OnComponentBeginOverlap(Box)
  (params (OverlappedComponent :type Primitive%20Component%20Object%20Reference) (OtherActor :type Actor%20Object%20Reference) (OtherComp :type Primitive%20Component%20Object%20Reference) (OtherBodyIndex :type Integer) (bFromSweep :type Boolean) (SweepResult :type Hit%20Result%20Structure%20%28by%20ref%29))
  (CallFunction|TEstOverlap OtherActor))

(event Custom|TEstOverlap
  (params (OverlappedActor :type Actor%20Object%20Reference))
  (bind _astest_actor_02 (Utilities|Casting|CastToTestActor02 OverlappedActor))
  (Variables|Default|SetSphereREF _astest_actor_02)
  (bind _asbp_first_person_character (Utilities|Casting|CastToBP_FirstPersonCharacter (Game|GetPlayerCharacter 0)))
  (if (not (Variables|Default|GetIsGrabbed))
    (if (not (Variables|/Game/Blueprints/TestActor02.TestActor02_C|GetIsGrabbed _astest_actor_02))
      (Physics|SetSimulatePhysics (Variables|/Game/Blueprints/TestActor02.TestActor02_C|GetSPhere _astest_actor_02) false)
      (Variables|/Game/XRFramework/Blueprints/BP_GrabComponent.BP_GrabComponent_C|SetGrabType (Variables|/Game/Blueprints/TestActor02.TestActor02_C|GetBP_GrabComponent _astest_actor_02) "NewEnumerator0")
      (Collision|SetCollisionEnabled (Variables|/Game/Blueprints/TestActor02.TestActor02_C|GetSPhere _astest_actor_02) "NoCollision")
      (Variables|Default|SetCollisionEnabled true)
      (Transformation|AttachComponentToComponent _astest_actor_02 (Variables|Default|GetSnapPoint_Top) "None" "SnapToTarget" "SnapToTarget" "KeepWorld" true))))

(event EventBeginPlay)

(event EventTick
  (params (DeltaSeconds :type Float%20%28single-precision%29)))

(event EventOnCustomerInteracted
  (Utilities|FlowControl|FlipFlop
    (:A
      (Variables|Default|SetIsGrabbed true)
      (Development|PrintString "IsGrabbed = True"))
    (:B
      (Variables|Default|SetIsGrabbed false)
      (Development|PrintString "IsGrabbed = False"))))

(fn ConstructionScript)

(fn OnRepCollisionEnabled
  (bind _sphereref (Variables|Default|GetSphereREF))
  (bind _sphere (Variables|/Game/Blueprints/TestActor02.TestActor02_C|GetSPhere _sphereref))
  (if (Utilities|IsValid _sphereref)
    (Development|PrintString "Hello")
    (Physics|SetSimulatePhysics _sphere false)
    (Collision|SetCollisionEnabled _sphere "NoCollision")))