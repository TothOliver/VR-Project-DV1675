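; BP_PhysicalButton is a button whose cap moves in while something overlaps its PressVolume and returns when the overlap ends.
; Begin and end overlap events set the Pressing flag, with no filtering or overlap counting.
; Tick eases the cap with VInterpTo between its BeginPlay position and a PressDistance offset along negative local Y, using separate press and release speeds.
; The button only animates and triggers no other logic.
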(event OnComponentBeginOverlap(PressVolume)
  (params (OverlappedComponent :type Primitive%20Component%20Object%20Reference) (OtherActor :type Actor%20Object%20Reference) (OtherComp :type Primitive%20Component%20Object%20Reference) (OtherBodyIndex :type Integer) (bFromSweep :type Boolean) (SweepResult :type Hit%20Result%20Structure%20%28by%20ref%29))
  (Variables|Default|SetbPressing true))

(event OnComponentEndOverlap(PressVolume)
  (params (OverlappedComponent :type Primitive%20Component%20Object%20Reference) (OtherActor :type Actor%20Object%20Reference) (OtherComp :type Primitive%20Component%20Object%20Reference) (OtherBodyIndex :type Integer))
  (Variables|Default|SetbPressing false))

(event EventBeginPlay
  ;[0.15 0.15 0.15 0.5] Sets up the state of the original unpressed button
  (bind _output_get (Variables|Default|SetStartRelLoc (Variables|/Script/Engine.SceneComponent|GetRelativeLocation (Variables|Default|GetButtonCap))))
  (Variables|Default|SetTargetRelLoc _output_get)
  (Variables|Default|SetbPressing false)
  (Transformation|SetRelativeLocation (Variables|Default|GetButtonCap) (Variables|Default|GetStartRelLoc) false false))

(event Collision|EventActorBeginOverlap
  (params (OtherActor :type Actor%20Object%20Reference)))

(event EventTick
  (params (DeltaSeconds :type Float%20%28single-precision%29))
  ;[0.15 0.15 0.15 0.5] Handles the locationshifting if the button is pressed down, and the logic that makes it go back to its orignial state(True moves it, False resets it)
  (if (Variables|Default|GetbPressing)
    (Variables|Default|SetTargetRelLoc (+ (Variables|Default|GetStartRelLoc) (Math|Vector|MakeVector 0.0 (* (Variables|Default|GetPressDistance) -1.0) 0.0)))
    (else
      (Variables|Default|SetTargetRelLoc (Variables|Default|GetStartRelLoc))))
  (Transformation|SetRelativeLocation (Variables|Default|GetButtonCap) (Math|Interpolation|VInterpTo (Variables|/Script/Engine.SceneComponent|GetRelativeLocation (Variables|Default|GetButtonCap)) (Variables|Default|GetTargetRelLoc) DeltaSeconds (Math|Float|SelectFloat (Variables|Default|GetPressSpeed) (Variables|Default|GetReleaseSpeed) (Variables|Default|GetbPressing))) false false))

(fn ConstructionScript)