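; BP_PotatoSpawner is an actor that spawns grabbable potatoes when its linked button is pressed.
; On BeginPlay it validates the button reference and binds to its pressed and repeat events, so holding the button keeps spawning.
; Both handlers call SpawnPotato, which creates a BP_GrabPotato at the SpawnPoint component's transform, always spawning regardless of collision.
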(event Custom|SpawnPotato
  ;[0.15 0.15 0.15 0.5] SpawnPotato function
  (Game|SpawnActorfromClass "/Game/Blueprints/BP_GrabPotato.BP_GrabPotato_C" (Transformation|GetWorldTransform (Variables|Default|GetSpawnPoint)) "AlwaysSpawn" "MultiplyWithRoot" 0 0))

(event Custom|HandleButtonPressed
  ;[0.15 0.15 0.15 0.5] Calls the Spawnpotato function on pressed and repeats it if its held down
  (CallFunction|SpawnPotato))

(event Custom|HandleButtonRepeat
  ;[0.15 0.15 0.15 0.5] Calls the Spawnpotato function on pressed and repeats it if its held down
  (CallFunction|SpawnPotato))

(event EventBeginPlay
  ;[0.15 0.15 0.15 0.5] Calls the Spawnpotato function on pressed and repeats it if its held down
  (Utilities|IsValid (Variables|Default|GetButtonRef)
    (:Is%20Valid
      (EventDispatchers|BindEventtoOnPressed (Variables|Default|GetButtonRef) (delegate Custom|HandleButtonPressed))
      (EventDispatchers|BindEventtoOnRepeat (Variables|Default|GetButtonRef) (delegate Custom|HandleButtonRepeat)))))

(event Collision|EventActorBeginOverlap
  (params (OtherActor :type Actor%20Object%20Reference)))

(event EventTick
  (params (DeltaSeconds :type Float%20%28single-precision%29)))

(fn ConstructionScript)